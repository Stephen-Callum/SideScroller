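; Floor button for a side-scroller that fires the SetElevatorEnabled dispatcher when the player character overlaps its trigger.
; A timeline squashes the button's Z scale, and its update disables trigger collision so the press happens only once.
; The same update turns the construction-script dynamic material green, zeroes its Frequency parameter and calls the dispatcher, so these repeat on every timeline tick.
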(event `self.ButtonTrigger.OnComponentBeginOverlap`
  (params (OverlappedComponent :type "PrimitiveComponent Object Reference") (OtherActor :type "Actor Object Reference") (OtherComp :type "PrimitiveComponent Object Reference") (OtherBodyIndex :type Integer) (bFromSweep :type Boolean) (SweepResult :type "HitResult Structure (by ref)"))
  (bind _btndynamicmaterialinstance (`self.btnDynamicMaterialInstance`))
  (bind (_returnvalue_x _returnvalue_y _returnvalue_z) (`KismetMathLibrary.BreakVector` (`SceneComponent.K2_GetComponentScale` (`self.Button`))))
  (bind _asside_scroller_character_bp (cast `/Game/Blueprints/SideScrollerCharacter_BP` OtherActor))
  (`/Engine/EditorBlueprintResources/StandardMacros.IsValid` _asside_scroller_character_bp
    (:`Is Valid`
      (bind (_direction _buttonscale) (`Timeline|ButtonScale`)
        (:`Update`
          (`SceneComponent.SetWorldScale3D` (`self.Button`) (`KismetMathLibrary.VLerp` (`KismetMathLibrary.MakeVector` _returnvalue_x _returnvalue_y _returnvalue_z) (`KismetMathLibrary.MakeVector` _returnvalue_x _returnvalue_y 0.35) _buttonscale))
          (`PrimitiveComponent.SetCollisionEnabled` (`self.ButtonTrigger`) "NoCollision")
          (`MaterialInstanceDynamic.SetVectorParameterValue` _btndynamicmaterialinstance "Color" (make `LinearColor` 0.0 3.0 0.0 1.0))
          (`MaterialInstanceDynamic.SetScalarParameterValue` _btndynamicmaterialinstance "Frequency" 0.0)
          (`self.SetElevatorEnabled` self))))))

(fn `UserConstructionScript`
  (bind _button (`self.Button`))
  (bind _returnvalue (`PrimitiveComponent.CreateDynamicMaterialInstance` _button 0 "/Game/Materials/E_Button.E_Button" "None"))
  (bind _output_get (set `self.btnDynamicMaterialInstance` _returnvalue))
  (`PrimitiveComponent.SetMaterial` _button 0 _output_get))