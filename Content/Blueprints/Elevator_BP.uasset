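; Elevator actor that oscillates up and down continuously while the game runs.
; Each Tick adds the change in the sine of accumulated running time, scaled by ElevationRate, to the current location and applies the new Z through SetActorLocation.
; The motion has no trigger or stop condition, and the construction script is empty.
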(event `self.ReceiveTick`
  (params (DeltaSeconds :type "Float (single-precision)"))
  (bind _runningtime (`self.RunningTime`))
  (set `self.NewLocation` (`self.K2_GetActorLocation`))
  (bind _output_get (set `self.DeltaHeight` (- (`KismetMathLibrary.Sin` (+ _runningtime DeltaSeconds)) (`KismetMathLibrary.Sin` _runningtime))))
  (bind _output_get_2 (set `self.NewLocation` (+ (`self.NewLocation`) (* _output_get (`self.ElevationRate`)))))
  (set `self.RunningTime` (+ (`self.RunningTime`) DeltaSeconds))
  (`self.K2_SetActorLocation` (`KismetMathLibrary.MakeVector` 0.0 0.0 (.z _output_get_2))))

(fn `UserConstructionScript`)