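; Teleporter actor that moves the side-scroller character to an exit actor, TeleportPoint, which can be changed through an event.
; On overlap it calls the character's enter hook, plays a sound, then teleports and calls the exit hook after short delays.
; A FlipFlop, duplicated in an event and a function, toggles trigger and mesh collision, feeding one boolean to hidden state, tick and debug prints.
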(event `self.ReceiveBeginPlay`
  ;[1 1 1] Bind events to dispatchers
  (add `self.SetTeleporterExit` (delegate `SetTeleporterExit_Event`))
  (add `self.SetTeleporterEnabled_Event` (delegate `SetTeleporterEnabledEvent`)))

(event `SetTeleporterExit_Event` :!signature `self.SetTeleporterExit`
  (params (TeleporterExit :type "Actor Object Reference"))
  ;[1 1 1] Bind events to dispatchers
  (set `self.TeleportPoint` TeleporterExit))

(event `SetTeleporterEnabledEvent`
  (bind _teleportercollision (`self.TeleporterCollision`))
  (bind _entrancemesh (`self.EntranceMesh`))
  ;[1 1 1] Bind events to dispatchers
  ;[1 1 1] Handle teleporter enabling/disabling
  (bind _isa (`/Engine/EditorBlueprintResources/StandardMacros.FlipFlop`)
    (:`A`
      (bind _output_get (set `self.CollisionParameterEnum` "NoCollision"))
      (`PrimitiveComponent.SetCollisionEnabled` _teleportercollision _output_get)
      (`PrimitiveComponent.SetCollisionEnabled` _entrancemesh _output_get))
    (:`B`
      (bind _output_get_2 (set `self.CollisionParameterEnum` "QueryOnly"))
      (`PrimitiveComponent.SetCollisionEnabled` _teleportercollision _output_get_2)
      (`PrimitiveComponent.SetCollisionEnabled` _entrancemesh _output_get_2)))
  (`self.SetActorHiddenInGame` _isa)
  (`self.SetActorTickEnabled` _isa)
  (`KismetSystemLibrary.PrintString` (`KismetStringLibrary.Conv_BoolToString` _isa))
  (`KismetSystemLibrary.PrintString` (`KismetStringLibrary.Conv_BoolToString` _isa)))

(event `self.TeleporterCollision.OnComponentBeginOverlap`
  (params (OverlappedComponent :type "PrimitiveComponent Object Reference") (OtherActor :type "Actor Object Reference") (OtherComp :type "PrimitiveComponent Object Reference") (OtherBodyIndex :type Integer) (bFromSweep :type Boolean) (SweepResult :type "HitResult Structure (by ref)"))
  (bind (_returnvalue_location _returnvalue_rotation) (`KismetMathLibrary.BreakTransform` (`self.GetTransform` (`self.TeleportPoint`))))
  ;[1 1 1] Handle Player Teleportation
  (bind _asside_scroller_character_bp (cast `/Game/Blueprints/SideScrollerCharacter_BP` OtherActor))
  (`/Engine/EditorBlueprintResources/StandardMacros.IsValid` _asside_scroller_character_bp
    (:`Is Valid`
      (`/Game/Blueprints/SideScrollerCharacter_BP.OnTelerporterEnter` _asside_scroller_character_bp)
      (`GameplayStatics.PlaySound2D` "/Game/Sounds/TeleportSoundCue.TeleportSoundCue" 1.0 1.0 0.0 null null)
      (`KismetSystemLibrary.Delay` 2.0)
      (`self.K2_TeleportTo` _asside_scroller_character_bp _returnvalue_location _returnvalue_rotation)
      (`KismetSystemLibrary.Delay` 0.5)
      (`/Game/Blueprints/SideScrollerCharacter_BP.OnTeleportExit` _asside_scroller_character_bp))))

(fn `SetTeleporterEnabled`
  (bind _teleportercollision (`self.TeleporterCollision`))
  (bind _entrancemesh (`self.EntranceMesh`))
  (bind _isa (`/Engine/EditorBlueprintResources/StandardMacros.FlipFlop`)
    (:`A`
      (bind _output_get (set `self.CollisionParameterEnum` "NoCollision"))
      (`PrimitiveComponent.SetCollisionEnabled` _teleportercollision _output_get)
      (`PrimitiveComponent.SetCollisionEnabled` _entrancemesh _output_get))
    (:`B`
      (bind _output_get_2 (set `self.CollisionParameterEnum` "QueryOnly"))
      (`PrimitiveComponent.SetCollisionEnabled` _teleportercollision _output_get_2)
      (`PrimitiveComponent.SetCollisionEnabled` _entrancemesh _output_get_2)))
  (`self.SetActorHiddenInGame` _isa)
  (`self.SetActorTickEnabled` _isa)
  (`KismetSystemLibrary.PrintString` (`KismetStringLibrary.Conv_BoolToString` _isa))
  (`KismetSystemLibrary.PrintString` (`KismetStringLibrary.Conv_BoolToString` _isa)))

(fn `UserConstructionScript`)