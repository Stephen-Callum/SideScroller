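; Key is a keycard pickup actor that spins in place and reacts to the side-scroller player character.
; Each tick, KeyMesh rotates on all three axes at fractions of RotationSpeed, scaled by delta time.
; On overlap with SideScrollerCharacter_BP it plays a 2D pickup sound; this graph neither grants the key nor removes the actor.
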(event `self.ReceiveActorBeginOverlap`
  (params (OtherActor :type "Actor Object Reference"))
  (bind _asside_scroller_character_bp (cast `/Game/Blueprints/SideScrollerCharacter_BP` OtherActor))
  (`/Engine/EditorBlueprintResources/StandardMacros.IsValid` _asside_scroller_character_bp
    (:`Is Valid`
      (`GameplayStatics.PlaySound2D` "/Game/Sounds/KeycardPickupCue.KeycardPickupCue" 1.0 1.0 0.0 null null))))

(event `self.ReceiveTick`
  (params (DeltaSeconds :type "Float (single-precision)"))
  (bind _rotationspeed (`self.RotationSpeed`))
  (`SceneComponent.K2_AddWorldRotation` (`self.KeyMesh`) (* (`KismetMathLibrary.MakeRotator` (/ _rotationspeed 4.0) (/ _rotationspeed 2.0) _rotationspeed) DeltaSeconds) false false))

(fn `UserConstructionScript`)